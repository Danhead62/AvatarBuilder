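; Test-bench Blueprint for a modular female avatar that swaps clothing and previews body morphs.
; Modular meshes follow Body via leader pose; BeginPlay plays an idle montage, caches populated meshes and opens the test widget.
; SetBottoms applies clothing and body meshes from a DataTable row, then refreshes morphing.
; One slider value drives two opposing morph targets around a neutral midpoint, plus Body's normal-map blending.
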(event Custom|Morphing
  (bind _fullbody (Variables|Default|GetFullBody))
  (bind _varmorphvalueinput (Variables|Default|GetVarMorphValueInput))
  ;[1 0 0 1 24] Temp Morphing Shitty Test
  (if (< _varmorphvalueinput 0.5)
    (Variables|Default|SetVarArrayNumber 0)
    (Variables|Default|SetVarMorphValue (Math|Float|MapRangeClamped (Variables|Default|GetVarMorphValueInput) 0.5 0.0 0.0 1.0))
    (for _array_element (Variables|Default|GetSMKArray) :!label _label
      (Components|SkeletalMesh|SetMorphTarget _array_element (Utilities|Array|Get(acopy) (Variables|Default|GetVarBodyMorphsArray) (Variables|Default|GetVarArrayNumber)) (Variables|Default|GetVarMorphValue) true)
      (Components|SkeletalMesh|SetMorphTarget _fullbody (Utilities|Array|Get(acopy) (Variables|Default|GetVarBodyMorphsArray_0) (Variables|Default|GetVarArrayNumber)) (Variables|Default|GetVarMorphValue) true)
      (Components|SkeletalMesh|SetMorphTarget _fullbody (Utilities|Array|Get(acopy) (Variables|Default|GetVarBodyMorphsArray_1) (Variables|Default|GetVarArrayNumber)) 0.0 true))
    (Rendering|Material|SetScalarParameterValue (Variables|Default|GetVarBodyDMI) "VarNormalMapBlending" (Variables|Default|GetVarMorphValueInput) :!class /Script/Engine.MaterialInstanceDynamic)
    (elif (> _varmorphvalueinput 0.5)
      (Variables|Default|SetVarArrayNumber 1)
      (Variables|Default|SetVarMorphValue (Math|Float|MapRangeClamped (Variables|Default|GetVarMorphValueInput) 0.5 1.0 0.0 1.0))
      (goto _label)
      (else
        (Variables|Default|SetVarMorphValue 0.0)
        (for _index (range 0 1)
          (Variables|Default|SetVarArrayNumber _index)
          (goto _label))))))

(event Custom|DoSomeShit
  ;[1 0 0 1 48] Clothes Normal Blending or some retarded crap
)

(event Custom|DoMoreShit
  (bind _varmata (Variables|Default|GetVarMatA))
  ;[1 0 0 1 48] Clothes Normal Blending or some retarded crap
  (for _index (range 0 (- (Utilities|Array|Length _varmata) 1))
    (Rendering|Material|SetScalarParameterValue (Utilities|Array|Get(acopy) _varmata _index) "VarNormalMapBlending" (Variables|Default|GetVarMorphValueInput) :!class /Script/Engine.MaterialInstanceDynamic)))

(event Custom|TattoTest
  (params (NewParam :type Integer))
  (bind _value (Variables|Default|GetValue))
  (bind (_r _g _b _a) (Utilities|Struct|BreakLinearColor _value))
  ;[1 0 0 1 48] Stupid Retarded Shit
  (switch int NewParam
    (:0
      (if (>= _r 1.0)
        (Variables|Default|SetNewVarR 0.0)
        (else
          (Variables|Default|SetNewVarR (+ _r 0.1)))))
    (:1
      (if (>= _g 1.0)
        (Variables|Default|SetNewVarG 0.0)
        (else
          (Variables|Default|SetNewVarG (+ _g 0.1)))))
    (:2
      (if (>= _b 1.0)
        (Variables|Default|SetNewVarB 0.0)
        (else
          (Variables|Default|SetNewVarB (+ _b 0.1)))))
    (:3
      (if (>= _a 1.0)
        (Variables|Default|SetNewVarA 0.0)
        (else
          (Variables|Default|SetNewVarA (+ _a 0.1))))))
  (Utilities|Struct|SetmembersinLinearColor _value (Variables|Default|GetNewVarR) (Variables|Default|GetNewVarG) (Variables|Default|GetNewVarB) (Variables|Default|GetNewVarA))
  (Rendering|Material|SetVectorParameterValue (Variables|Default|GetNewVar) "VarTattooHeadColor01" _value :!class /Script/Engine.MaterialInstanceDynamic)
  (Development|PrintString (Utilities|String|ToString(Integer) _value)))

(event Custom|PrintMorphValue
  ;[0 0 0 1 24] Event Begin Play - Print Morph Value Every 0.5 Seconds
)

(event Custom|MorphValueChange
  (params (bIncrease :type Boolean))
  (if bIncrease
    (Variables|Default|SetVarMorphValueInput (Math|Float|Max(Float) (- (Variables|Default|GetVarMorphValueInput) 0.1) 0.0))
    (else
      (Variables|Default|SetVarMorphValueInput (Math|Float|Min(Float) (+ (Variables|Default|GetVarMorphValueInput) 0.1) 1.0))))
  (CallFunction|Morphing))

(event Custom|BuildSMKArray
  ;[0 0 0 1 24] Build Skeletal Mesh Array
  (for _array_element (Utilities|Array|MakeArray (Variables|Default|GetBottoms) (Variables|Default|GetShoes) (Variables|Default|GetHair) (Variables|Default|GetEars) (Variables|Default|GetNeck) (Variables|Default|GetFace) (Variables|Default|GetFullBody) (Variables|Default|GetArm) (Variables|Default|GetBack) (Variables|Default|GetHeadTop) (Variables|Default|GetTop) (Variables|Default|GetBody))
    (Utilities|IsValid (Class|SkinnedMeshComponent|GetSkinnedAsset _array_element)
      (:Is%20Valid
        (Utilities|Array|Add (Variables|Default|GetSMKArray) _array_element)))))

(event Custom|PlayANimation
  ;[0 0 0 1 24] Event Begin Play - Print Morph Value Every 0.5 Seconds
  (Animation|Montage|PlayMontage (Variables|Default|GetBody) "/ShibAvatarBuilder/Assets/AvatarAssets/FemBodyAssets/AM_TempFemIdle.AM_TempFemIdle"))

(event Custom|SetupTable
  (bind _returnvalue (Game|GetPlayerController 0))
  (bind _returnvalue_2 (UserInterface|CreateWidget "/Game/AvatarAssets/NoelWeightPaintTest/Test01/WB_TestBenchFem.WB_TestBenchFem_C"))
  (UserInterface|Viewport|AddtoViewport _returnvalue_2 0)
  (Input|SetInputModeGameandUI _returnvalue _returnvalue_2 "DoNotLock" true false)
  (Variables|/Script/Engine.PlayerController|SetbShowMouseCursor _returnvalue true))

(event Custom|SetBottoms
  (params (RowName :type Name))
  (bind _returnvalue (Utilities|GetDataTableRow "/Game/AvatarAssets/NoelWeightPaintTest/Test01/DT_TestBenchFem.DT_TestBenchFem" RowName)
    (:then
      (Utilities|FlowControl|Sequence
        (:then_0
          (if (== (.clothesindex _returnvalue) 0)
            (Components|SkinnedMesh|SetSkinnedAssetandUpdate (Variables|Default|GetBottoms) (.clothes _returnvalue) false)
            (Components|SkinnedMesh|SetSkinnedAssetandUpdate (Variables|Default|GetFullBody) 0 false :!label _label)
            (Components|SkinnedMesh|SetSkinnedAssetandUpdate (Variables|Default|GetBody) (.bodyoptions _returnvalue) false :!label _label_2)
            (CallFunction|Morphing)))
        (:then_1
          (if (== (.clothesindex _returnvalue) 1)
            (Components|SkinnedMesh|SetSkinnedAssetandUpdate (Variables|Default|GetTop) (.clothes _returnvalue) false)
            (goto _label)))
        (:then_2
          (if (== (.clothesindex _returnvalue) 2)
            (Components|SkinnedMesh|SetSkinnedAssetandUpdate (Variables|Default|GetFullBody) (.clothes _returnvalue) false)
            (Components|SkinnedMesh|SetSkinnedAssetandUpdate (Variables|Default|GetBottoms) 0 false)
            (goto _label_2)))
        (:then_3
          (if (== (.clothesindex _returnvalue) 3)
            (Components|SkinnedMesh|SetSkinnedAssetandUpdate (Variables|Default|GetBottoms) (.clothes _returnvalue) false)
            (goto _label)))))))

(event EventBeginPlay
  ;[0 0 0 1 24] Event Begin Play - Print Morph Value Every 0.5 Seconds
  (Variables|Default|SetVarMorphValueInput 0.5)
  (CallFunction|PlayANimation)
  (CallFunction|BuildSMKArray)
  (CallFunction|CaptureBodyDynamicMaterial)
  (Utilities|Time|SetTimerbyFunctionName 0 "PrintMorphValue" 1.0 true true)
  (CallFunction|SetupTable))

(fn ConstructionScript
  (Components|SkinnedMesh|SetLeaderPoseComponent (Variables|Default|GetShoes) (Variables|Default|GetBody) false false))

(fn CaptureBodyDynamicMaterial
  (bind _body (Variables|Default|GetBody))
  (bind _returnvalue (Rendering|Material|CreateDynamicMaterialInstance _body 0 (Rendering|Material|GetMaterial _body 0) "None" :!class /Script/Engine.PrimitiveComponent))
  (Variables|Default|SetVarBodyDMI _returnvalue))