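; Test Blueprint for a modular female avatar that tries out body morphing and tattoo tinting.
; The construction script makes clothing, hair and other parts follow the Body's pose.
; MorphValueChange steps a slider around a 0.5 neutral, driving two opposing morph targets across all populated meshes and normal-map blending on the Body's dynamic material.
; A debug timer prints the morph value; TattoTest's material setup is disconnected.
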(event Custom|Morphing
  (bind _varmorphvalueinput (Variables|Default|GetVarMorphValueInput))
  ;[1 0 0 1 24] Temp Morphing Shitty Test
  (if (< _varmorphvalueinput 0.5)
    (Variables|Default|SetVarArrayNumber 0)
    (Variables|Default|SetVarMorphValue (Math|Float|MapRangeClamped (Variables|Default|GetVarMorphValueInput) 0.5 0.0 0.0 1.0))
    (for _array_element (Variables|Default|GetSMKArray) :!label _label
      (Components|SkeletalMesh|SetMorphTarget _array_element (Utilities|Array|Get(acopy) (Variables|Default|GetVarBodyMorphsArray) (Variables|Default|GetVarArrayNumber)) (Variables|Default|GetVarMorphValue) true))
    (Rendering|Material|SetScalarParameterValue (Variables|Default|GetVarBodyDMI) "VarNormalMapBlending" (Variables|Default|GetVarMorphValueInput) :!class /Script/Engine.MaterialInstanceDynamic)
    (elif (> _varmorphvalueinput 0.5)
      (Variables|Default|SetVarArrayNumber 1)
      (Variables|Default|SetVarMorphValue (Math|Float|MapRangeClamped (Variables|Default|GetVarMorphValueInput) 0.5 1.0 0.0 1.0))
      (goto _label)
      (else
        (Variables|Default|SetVarMorphValue 0.0)
        (for _index (range 0 1)
          (Variables|Default|SetVarArrayNumber _index)
          (goto _label))))))

(event Custom|DoSomeShit
  ;[1 0 0 1 48] Clothes Normal Blending or some retarded crap
)

(event Custom|DoMoreShit
  (bind _varmata (Variables|Default|GetVarMatA))
  ;[1 0 0 1 48] Clothes Normal Blending or some retarded crap
  (for _index (range 0 (- (Utilities|Array|Length _varmata) 1))
    (Rendering|Material|SetScalarParameterValue (Utilities|Array|Get(acopy) _varmata _index) "VarNormalMapBlending" (Variables|Default|GetVarMorphValueInput) :!class /Script/Engine.MaterialInstanceDynamic)))

(event Custom|TattoTest
  (params (NewParam :type Integer))
  (bind _value (Variables|Default|GetValue))
  (bind (_r _g _b _a) (Utilities|Struct|BreakLinearColor _value))
  ;[1 0 0 1 48] Stupid Retarded Shit
  (switch int NewParam
    (:0
      (if (>= _r 1.0)
        (Variables|Default|SetNewVarR 0.0)
        (else
          (Variables|Default|SetNewVarR (+ _r 0.1)))))
    (:1
      (if (>= _g 1.0)
        (Variables|Default|SetNewVarG 0.0)
        (else
          (Variables|Default|SetNewVarG (+ _g 0.1)))))
    (:2
      (if (>= _b 1.0)
        (Variables|Default|SetNewVarB 0.0)
        (else
          (Variables|Default|SetNewVarB (+ _b 0.1)))))
    (:3
      (if (>= _a 1.0)
        (Variables|Default|SetNewVarA 0.0)
        (else
          (Variables|Default|SetNewVarA (+ _a 0.1))))))
  (Utilities|Struct|SetmembersinLinearColor _value (Variables|Default|GetNewVarR) (Variables|Default|GetNewVarG) (Variables|Default|GetNewVarB) (Variables|Default|GetNewVarA))
  (Rendering|Material|SetVectorParameterValue (Variables|Default|GetNewVar) "VarTattooHeadColor01" _value :!class /Script/Engine.MaterialInstanceDynamic)
  (Development|PrintString (Utilities|String|ToString(Integer) _value)))

(event Custom|PrintMorphValue
  ;[0 0 0 1 24] Event Begin Play - Print Morph Value Every 0.5 Seconds
  (Development|PrintString (Utilities|String|ToString(Float) (Variables|Default|GetVarMorphValue)) true true "(R=1.000000,G=0.000000,B=0.000000,A=1.000000)"))

(event Custom|MorphValueChange
  (params (bIncrease :type Boolean))
  (if bIncrease
    (Variables|Default|SetVarMorphValueInput (Math|Float|Max(Float) (- (Variables|Default|GetVarMorphValueInput) 0.1) 0.0))
    (else
      (Variables|Default|SetVarMorphValueInput (Math|Float|Min(Float) (+ (Variables|Default|GetVarMorphValueInput) 0.1) 1.0))))
  (CallFunction|Morphing))

(event Custom|BuildSMKArray
  ;[0 0 0 1 24] Event Begin Play - Print Morph Value Every 0.5 Seconds
  (for _array_element (Utilities|Array|MakeArray (Variables|Default|GetBottoms) (Variables|Default|GetShoes) (Variables|Default|GetHair) (Variables|Default|GetEars) (Variables|Default|GetNeck) (Variables|Default|GetFace) (Variables|Default|GetFullBody) (Variables|Default|GetArm) (Variables|Default|GetBack) (Variables|Default|GetHeadTop) (Variables|Default|GetTop) (Variables|Default|GetBody))
    (Utilities|IsValid (Class|SkinnedMeshComponent|GetSkinnedAsset _array_element)
      (:Is%20Valid
        (Utilities|Array|Add (Variables|Default|GetSMKArray) _array_element)))))

(event EventBeginPlay
  ;[0 0 0 1 24] Event Begin Play - Print Morph Value Every 0.5 Seconds
  (Variables|Default|SetVarMorphValueInput 0.5)
  (Utilities|Time|SetTimerbyFunctionName 0 "PrintMorphValue" 0.5 true)
  (CallFunction|BuildSMKArray)
  (CallFunction|CaptureBodyDynamicMaterial))

(fn ConstructionScript
  (Components|SkinnedMesh|SetLeaderPoseComponent (Variables|Default|GetShoes) (Variables|Default|GetBody) false false))

(fn CaptureBodyDynamicMaterial
  (bind _body (Variables|Default|GetBody))
  (bind _returnvalue (Rendering|Material|CreateDynamicMaterialInstance _body 0 (Rendering|Material|GetMaterial _body 0) "None" :!class /Script/Engine.PrimitiveComponent))
  (Variables|Default|SetVarBodyDMI _returnvalue))